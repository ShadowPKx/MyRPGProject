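; Player hero character with a toggleable lightsaber, random melee attacks, damage handling and respawn at its start location.
; Input toggles the saber child actor's visibility, collision and armed state, and plays attack montages under sped-up global time.
; AdvancedMovementComponent holds combat flags, while CharacteristicsComponent holds health, which drives a timed death-and-respawn sequence.
; It also creates the HUD, switches inventory and menu states through InventoryGameMode, and prints debug stats on Tick.
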(event `InputAction|Hide/Show Weapon`
  (params (Key :type "Key Structure"))
  (bind _lightsaber_bp (`self.Lightsaber_BP`))
  (bind _advancedmovementcomponent (`self.AdvancedMovementComponent`))
  (bind _aslightsaber (cast `Lightsaber` (`ChildActorComponent.ChildActor` _lightsaber_bp) :!pure true))
  (bind _saber_collision (`Lightsaber.Saber_Collision` _aslightsaber))
  ;[1 1 1] Активируем/деактивируем меч
  (:`Pressed`
    (if (`Lightsaber.Deactivate` _aslightsaber)
      (set `Lightsaber.Deactivate` false _aslightsaber)
      (`SceneComponent.ToggleVisibility` _lightsaber_bp true)
      (set `AdvancedMovementComponent.is_Armed` true _advancedmovementcomponent)
      (`PrimitiveComponent.SetCollisionProfileName` _saber_collision "OverlapAll")
      (else
        (set `Lightsaber.Deactivate` true _aslightsaber)
        (`SceneComponent.ToggleVisibility` _lightsaber_bp false)
        (set `AdvancedMovementComponent.is_Armed` false _advancedmovementcomponent)
        (`PrimitiveComponent.SetCollisionProfileName` _saber_collision "NoCollision")))))

(event `self.ReceiveBeginPlay`
  (bind _lightsaber_bp (`self.Lightsaber_BP`))
  ;[1 1 1] Устанавливаем HUD
  (bind _returnvalue (`|CreateWidget` "/Game/MyFiles/UI/HUD.HUD_C"))
  (`UserWidget.AddToViewport` _returnvalue 0)
  ;[1 1 1] Деактивируем меч в начале
  (set `Lightsaber.Deactivate` true (cast `Lightsaber` (`ChildActorComponent.ChildActor` _lightsaber_bp) :!pure true))
  ;[1 1 1] Если меч включен - выключаем его
  (if (`SceneComponent.IsVisible` _lightsaber_bp)
    (`SceneComponent.ToggleVisibility` _lightsaber_bp false)
    ;[1 1 1] Start info
    (set `self.Start Animation` (`SkeletalMeshComponent.GetAnimationMode` (`self.Mesh`)))
    (set `self.Start location` (`self.K2_GetActorLocation`))))

(event `self.ReceiveTick`
  (params (DeltaSeconds :type "Float (single-precision)"))
  (bind _advancedmovementcomponent (`self.AdvancedMovementComponent`))
  (bind _characteristicscomponent (`self.CharacteristicsComponent`))
  ;[1 1 1] Debug movement
  (`KismetSystemLibrary.PrintString` (`KismetStringLibrary.Concat_StrStr` "Speed:" (`KismetStringLibrary.Conv_DoubleToString` (`AdvancedMovementComponent.Speed` _advancedmovementcomponent))) false false (struct :`G` 0.66 :`B` 1.0 :`A` 1.0) 0.0)
  (`KismetSystemLibrary.PrintString` (`KismetStringLibrary.Concat_StrStr` "Input X:" (`KismetStringLibrary.Conv_DoubleToString` (`AdvancedMovementComponent.InputX` _advancedmovementcomponent))) false false (struct :`G` 0.66 :`B` 1.0 :`A` 1.0) 0.0)
  (`KismetSystemLibrary.PrintString` (`KismetStringLibrary.Concat_StrStr` "Input Z:" (`KismetStringLibrary.Conv_DoubleToString` (`AdvancedMovementComponent.InputZ` _advancedmovementcomponent))) false false (struct :`G` 0.66 :`B` 1.0 :`A` 1.0) 0.0)
  (`KismetSystemLibrary.PrintString` (`KismetStringLibrary.Concat_StrStr` "Direction:" (`KismetStringLibrary.Conv_DoubleToString` (`AdvancedMovementComponent.Direction` _advancedmovementcomponent))) false false (struct :`G` 0.66 :`B` 1.0 :`A` 1.0) 0.0)
  (`KismetSystemLibrary.PrintString` (`KismetStringLibrary.Concat_StrStr` "Health:" (`KismetStringLibrary.Conv_DoubleToString` (`CharacteristicsComponent.Health` (`self.CharacteristicsComponent`)))) false false (struct :`R` 0.093438 :`G` 1.0 :`A` 1.0) 0.0)
  (if (<= (`CharacteristicsComponent.Health` _characteristicscomponent) 0.0)
    (set `CharacteristicsComponent.Health` 1.0 _characteristicscomponent)))

(event `InputAction|Attack`
  (params (Key :type "Key Structure"))
  (bind _advancedmovementcomponent (`self.AdvancedMovementComponent`))
  (bind _advancedmovementcomponent_2 (`self.AdvancedMovementComponent`))
  ;[1 1 1] Attack motions
  (:`Pressed`
    (if (not (or (`AdvancedMovementComponent.is_Attacking` _advancedmovementcomponent_2) (not (`AdvancedMovementComponent.is_Armed` _advancedmovementcomponent_2))))
      (`GameplayStatics.SetGlobalTimeDilation` 1.5)
      (`|PlayMontage` (`self.Mesh`) (select `int` (`KismetMathLibrary.RandomIntegerInRange` 0 1) :`0` "/Game/MyFiles/MyAnimations/Combos/Great_Sword_Slash_Montage.Great_Sword_Slash_Montage" :`1` "/Game/MyFiles/MyAnimations/Combos/Sword_And_Shield_Slash__1__Montage.Sword_And_Shield_Slash__1__Montage" :!type "AnimMontage Object Reference")
        (:`then`
          (set `AdvancedMovementComponent.is_Attacking` true _advancedmovementcomponent))
        (:`OnCompleted`
          (set `AdvancedMovementComponent.is_Attacking` false _advancedmovementcomponent :!label _label)
          (`GameplayStatics.SetGlobalTimeDilation` 1.0))
        (:`OnInterrupted`
          (goto _label))))))

(event `self.ReceiveAnyDamage`
  (params (Damage :type "Float (single-precision)") (DamageType :type "DamageType Object Reference") (InstigatedBy :type "Controller Object Reference") (DamageCauser :type "Actor Object Reference"))
  (bind _characteristicscomponent (`self.CharacteristicsComponent`))
  (bind _lightsaber_bp (`self.Lightsaber_BP`))
  ;[1 1 1] Check and update health
  (bind _output_get (set `CharacteristicsComponent.Health` (- (`CharacteristicsComponent.Health` _characteristicscomponent) Damage) _characteristicscomponent))
  ;;[0.9323 0.1676 0] Debug
  (`KismetSystemLibrary.PrintString` (`KismetStringLibrary.Concat_StrStr` "Enemy health:" (`KismetStringLibrary.Conv_DoubleToString` _output_get)) false false (struct :`R` 0.431103 :`G` 1.0 :`B` 0.162381 :`A` 1.0))
  (if (<= _output_get 0.001)
    ;[1 1 1] При наступлении смерти
    ;;[1 1 1] Выключаем collision и дамаг
    (set `AdvancedMovementComponent.is_Alive` false (`self.AdvancedMovementComponent`))
    (`PrimitiveComponent.SetCollisionProfileName` (`self.Mesh`) "NoCollision")
    (set `self.bCanBeDamaged` false)
    ;;[1 1 1] Выключаем дамаг меча
    (set `self.JumpMaxCount` 0)
    (set `Lightsaber.Deactivate` true (cast `Lightsaber` (`ChildActorComponent.ChildActor` _lightsaber_bp) :!pure true))
    ;;[1 1 1] Проигрываем анимацию сметри
    (`SkeletalMeshComponent.PlayAnimation` (`self.Mesh`) "/Game/MyFiles/MyAnimations/Sword_And_Shield_Death.Sword_And_Shield_Death" false)
    ;;[1 1 1] Если меч включен - выключаем его
    (if (`SceneComponent.IsVisible` _lightsaber_bp)
      (`SceneComponent.ToggleVisibility` _lightsaber_bp false))
    ;[1 1 1] Respawn
    (`KismetSystemLibrary.Delay` 5.0)
    (set `AdvancedMovementComponent.is_Alive` true (`self.AdvancedMovementComponent`))
    (`self.K2_SetActorLocation` (`self.Start location`) false true)
    (`SkeletalMeshComponent.SetAnimationMode` (`self.Mesh`) (`self.Start Animation`))
    (set `CharacteristicsComponent.Health` 1.0 (`self.CharacteristicsComponent`))
    (`PrimitiveComponent.SetCollisionProfileName` (`self.Mesh`) "CharacterMesh")
    (set `self.bCanBeDamaged` true)
    (set `AdvancedMovementComponent.is_Armed` false (`self.AdvancedMovementComponent`))
    (set `self.JumpMaxCount` 1)))

(event `InputAction|ToggleInventory`
  (params (Key :type "Key Structure"))
  (bind _returnvalue (`GameplayStatics.GetPlayerController` 0))
  (bind _asinventory_game_mode (cast `/Game/MyFiles/Blueprints/InventoryGameMode` (`GameplayStatics.GetGameMode`) :!pure true))
  ;[1 1 1] Toggle Inventory
  (:`Pressed`
    (bind _returnvalue_2 (`MyProjectGameMode.GetHUDState` _asinventory_game_mode))
    (if (!= _returnvalue_2 1)
      (`MyProjectGameMode.ChangeHUDState` _asinventory_game_mode 1)
      (`Controller.SetIgnoreLookInput` _returnvalue true)
      (else
        (`MyProjectGameMode.ChangeHUDState` _asinventory_game_mode 0)
        (`Controller.SetIgnoreLookInput` _returnvalue false)))))

(event `InputAction|MenuMode`
  (params (Key :type "Key Structure"))
  (bind _returnvalue (`GameplayStatics.GetPlayerController` 0))
  (bind _asinventory_game_mode (cast `/Game/MyFiles/Blueprints/InventoryGameMode` (`GameplayStatics.GetGameMode`) :!pure true))
  ;[1 1 1] Toggle Menu
  (:`Pressed`
    (bind _returnvalue_2 (`MyProjectGameMode.GetHUDState` _asinventory_game_mode))
    (if (!= _returnvalue_2 4)
      (`MyProjectGameMode.ChangeHUDState` _asinventory_game_mode 4)
      (`Controller.SetIgnoreLookInput` _returnvalue true)
      (else
        (`MyProjectGameMode.ChangeHUDState` _asinventory_game_mode 0)
        (`Controller.SetIgnoreLookInput` _returnvalue false)))))

(fn `UserConstructionScript`)